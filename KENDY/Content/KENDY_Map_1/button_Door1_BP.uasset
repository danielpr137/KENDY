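; Button-operated door Blueprint that lets the player toggle a door open and closed when nearby.
; An interaction box overlap with BP_Player enables input and opens a Gate for the Crouch action.
; The press runs a button macro that alternately tilts the button via timeline, then a FlipFlop plays or reverses the door's position timeline.
; The construction script places the button from a transform variable.
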(event `InputAction|Crouch`
  (params (Key :type "Key Structure"))
  ;[1 1 1] Open door if player is close enough
  (:`Pressed`
    (`/Engine/EditorBlueprintResources/StandardMacros.Gate` true :!label _label
      (:`Exit`
        (`/Engine/EditorBlueprintResources/StandardMacros.FlipFlop`
          (:`A`
            (bind (_direction _button1_track) (`Timeline|Button1_Press` :!label _label_2)
              (:`Update`
                (`SceneComponent.K2_SetRelativeRotation` (`self.Button1`) (`KismetMathLibrary.MakeRotator` 0.0 (`KismetMathLibrary.Lerp` (`self.Button1 Up`) (`self.Button1 Down`) _button1_track)) false false))
              (:`Finished`
                ;[1 1 1] Open and close door
                (`/Engine/EditorBlueprintResources/StandardMacros.FlipFlop`
                  (:`A`
                    (bind (_direction_2 _door1_track) (`Timeline|Door1_Timeline` :!label _label_3)
                      (:`Update`
                        (`SceneComponent.K2_SetRelativeLocation` (`self.Door1`) (`KismetMathLibrary.VLerp` (`self.Door1_Closed`) (`self.Door1_Up`) _door1_track) false false))))
                  (:`B`
                    (goto _label_3 :!via `Reverse`))))))
          (:`B`
            (goto _label_2 :!via `Reverse`)))))))

(event `self.Interaction Box.OnComponentBeginOverlap`
  (params (OverlappedComponent :type "PrimitiveComponent Object Reference") (OtherActor :type "Actor Object Reference") (OtherComp :type "PrimitiveComponent Object Reference") (OtherBodyIndex :type Integer) (bFromSweep :type Boolean) (SweepResult :type "HitResult Structure (by ref)"))
  ;[1 1 1] Open door if player is close enough
  (cast `/Game/Blueprints/BP_Player` OtherActor)
  (`self.EnableInput` (`GameplayStatics.GetPlayerController` 0))
  (goto _label :!via `Open`))

(event `self.Interaction Box.OnComponentEndOverlap`
  (params (OverlappedComponent :type "PrimitiveComponent Object Reference") (OtherActor :type "Actor Object Reference") (OtherComp :type "PrimitiveComponent Object Reference") (OtherBodyIndex :type Integer))
  ;[1 1 1] Open door if player is close enough
  (cast `/Game/Blueprints/BP_Player` OtherActor)
  (`self.DisableInput` (`GameplayStatics.GetPlayerController` 0))
  (goto _label :!via `Close`))

(fn `UserConstructionScript`
  (`SceneComponent.K2_SetRelativeTransform` (`self.Button1`) (`self.Button Transform`) false false))